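; Main game mode that owns the projector UI and relays projector visibility changes.
; On BeginPlay it sets game-only input, creates WBP_ProjectorUI and passes itself to the widget.
; ShowUI toggles that widget on screen, switching input mode and mouse cursor to match.
; BroadcastShowProjector fires a dispatcher with the show/hide flag for any bound listeners.
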(event EventBeginPlay
  (Input|SetInputModeGameOnly (Game|GetPlayerController 0) false)
  (bind _returnvalue (UserInterface|CreateWidget "/Game/Blueprints/UI/WBP_ProjectorUI.WBP_ProjectorUI_C"))
  (Variables|Default|SetMainUI _returnvalue)
  (Default|SetGameMode (Variables|Default|GetMainUI) self))

(fn ConstructionScript)

(fn BroadcastShowProjector
  (params (ShouldShowProjector :type Boolean))
  (Default|CallProjectorDispatcher ShouldShowProjector))

(fn ShowUI
  (bind _returnvalue (Game|GetPlayerController 0))
  (bind _mainui (Variables|Default|GetMainUI))
  (if (Variables|Default|GetIsUIShowing)
    (Widget|RemovefromParent _mainui)
    (Input|SetInputModeGameOnly _returnvalue false)
    (Variables|/Script/Engine.PlayerController|SetbShowMouseCursor _returnvalue false)
    (Variables|Default|SetIsUIShowing false)
    (else
      (UserInterface|Viewport|AddtoViewport _mainui 0)
      (Input|SetInputModeGameandUI _returnvalue _mainui "DoNotLock" false false)
      (Variables|/Script/Engine.PlayerController|SetbShowMouseCursor _returnvalue true)
      (Variables|Default|SetIsUIShowing true))))