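; BP_Projector is a video projector actor that shows or hides a birds video on its plane when the game mode signals it.
; On BeginPlay it binds to BP_MainGameMode's projector dispatcher and opens the SMS_Birds media source, holding it paused at the start once loaded.
; Showing restarts playback and applies the video material.
; Hiding restores the basic shape material, then rewinds and pauses the player.
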(event Custom|OnMediaOpened
  (params (OpenedUrl :type String))
  (bind _mediaplayer (Variables|Default|GetMediaPlayer))
  (Class|MediaPlayer|Rewind _mediaplayer)
  (Sequencer|Player|Pause _mediaplayer))

(event Custom|ShowProjectorEvent
  (params (ShouldShowProjector :type Boolean))
  (bind _mediaplayer (Variables|Default|GetMediaPlayer))
  (bind _mediaplayer_2 (Variables|Default|GetMediaPlayer))
  (if ShouldShowProjector
    (Development|PrintString "Show Projector")
    (Class|MediaPlayer|Rewind _mediaplayer)
    (Media|MediaPlayer|Play _mediaplayer :!class /Script/MediaAssets.MediaPlayer)
    (Rendering|Material|SetMaterial (Variables|Default|GetPlane) 0 "/Game/Materials/M_VideoProjector.M_VideoProjector")
    (else
      (Development|PrintString "Hide Projector")
      (Rendering|Material|SetMaterial (Variables|Default|GetPlane) 0 "/Engine/BasicShapes/BasicShapeMaterial.BasicShapeMaterial")
      (Class|MediaPlayer|Rewind _mediaplayer_2)
      (Sequencer|Player|Pause _mediaplayer_2))))

(event EventBeginPlay
  (bind _mediaplayer (Variables|Default|GetMediaPlayer))
  (bind _asbp_main_game_mode (Utilities|Casting|CastToBP_MainGameMode (Game|GetGameMode)))
  (EventDispatchers|BindEventtoProjectorDispatcher _asbp_main_game_mode (delegate Custom|ShowProjectorEvent))
  (Media|MediaPlayer|OpenSource _mediaplayer "/Game/Video/SMS_Birds.SMS_Birds")
  (Media|MediaPlayer|BindEventtoOnMediaOpened _mediaplayer (delegate Custom|OnMediaOpened)))

(fn ConstructionScript)